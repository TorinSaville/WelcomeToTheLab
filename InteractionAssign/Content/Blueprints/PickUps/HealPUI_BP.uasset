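; HealPUI_BP is a health pickup that heals the third-person player character when touched.
; It polls for player overlap every Tick, with the ActorBeginOverlap event left disabled, and calls HealHealth with a fixed amount.
; A successful heal shows the HealGreenScreen_BP widget, destroys the pickup and increments pickup and healing totals on a TextFileManager found at BeginPlay.
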(event EventBeginPlay
  (|CallParentFunction)
  (bind _returnvalue (Actor|GetActorOfClass "/Game/Blueprints/TextFileManager/TextFileManager.TextFileManager_C"))
  (Variables|Default|SetTextFileManager _returnvalue))

(event Collision|EventActorBeginOverlap
  (params (OtherActor :type Actor%20Object%20Reference))
  (|CallParentFunction OtherActor) ; This node is disabled and will not be called.\nDrag off pins to build functionality.
)

(event EventTick
  (params (DeltaSeconds :type Float%20%28single-precision%29))
  (bind _returnvalue (Game|GetPlayerCharacter 0))
  (bind _textfilemanager (Variables|Default|GetTextFileManager))
  (|CallParentFunction DeltaSeconds)
  (if (Collision|IsOverlappingActor _returnvalue :!class /Script/Engine.Actor)
    (bind _asbp_third_person_character (Utilities|Casting|CastToBP_ThirdPersonCharacter _returnvalue))
    (bind _returnvalue_2 (Class|InteractionAssignCharacter|HealHealth _asbp_third_person_character 0.25))
    (if _returnvalue_2
      (bind _returnvalue_3 (UserInterface|CreateWidget "/Game/UI/Widgets/ScreenFlashes/HealGreenScreen_BP.HealGreenScreen_BP_C"))
      (UserInterface|Viewport|AddtoViewport _returnvalue_3 0)
      (Actor|DestroyActor)
      (Variables|/Game/Blueprints/TextFileManager/TextFileManager.TextFileManager_C|SetHealthPU _textfilemanager (+ (Variables|/Game/Blueprints/TextFileManager/TextFileManager.TextFileManager_C|GetHealthPU _textfilemanager) 1))
      (Variables|/Game/Blueprints/TextFileManager/TextFileManager.TextFileManager_C|SetHealthHealed _textfilemanager (+ (Variables|/Game/Blueprints/TextFileManager/TextFileManager.TextFileManager_C|GetHealthHealed _textfilemanager) 0.25)))))

(fn ConstructionScript
  (|CallParentFunction))