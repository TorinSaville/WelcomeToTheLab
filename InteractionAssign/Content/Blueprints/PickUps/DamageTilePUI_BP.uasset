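; DamageTilePUI_BP is a damage pickup tile that hurts the third-person player character once on contact, then destroys itself.
; It polls for overlap with the player on Tick, as the ActorBeginOverlap event is disabled.
; A hit applies a small fixed health loss, shows a red-screen damage widget, and updates the damage pickup count and damage total on a TextFileManager found at BeginPlay.
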(event EventBeginPlay
  (|CallParentFunction)
  (bind _returnvalue (Actor|GetActorOfClass "/Game/Blueprints/TextFileManager/TextFileManager.TextFileManager_C"))
  (Variables|Default|SetTextFileManager _returnvalue))

(event Collision|EventActorBeginOverlap
  (params (OtherActor :type Actor%20Object%20Reference))
  (|CallParentFunction OtherActor) ; This node is disabled and will not be called.\nDrag off pins to build functionality.
)

(event EventTick
  (params (DeltaSeconds :type Float%20%28single-precision%29))
  (bind _returnvalue (Game|GetPlayerCharacter 0))
  (bind _textfilemanager (Variables|Default|GetTextFileManager))
  (if (Collision|IsOverlappingActor _returnvalue :!class /Script/Engine.Actor)
    (bind _asbp_third_person_character (Utilities|Casting|CastToBP_ThirdPersonCharacter _returnvalue))
    (Class|InteractionAssignCharacter|DamageHealth _asbp_third_person_character 0.1)
    (bind _returnvalue_2 (UserInterface|CreateWidget "/Game/UI/Widgets/ScreenFlashes/DamageRedScreen_BP.DamageRedScreen_BP_C"))
    (UserInterface|Viewport|AddtoViewport _returnvalue_2 0)
    (Actor|DestroyActor)
    (Variables|/Game/Blueprints/TextFileManager/TextFileManager.TextFileManager_C|SetDamagePU _textfilemanager (+ (Variables|/Game/Blueprints/TextFileManager/TextFileManager.TextFileManager_C|GetDamagePU _textfilemanager) 1))
    (Variables|/Game/Blueprints/TextFileManager/TextFileManager.TextFileManager_C|SetDamageTaken _textfilemanager (+ (Variables|/Game/Blueprints/TextFileManager/TextFileManager.TextFileManager_C|GetDamageTaken _textfilemanager) 0.1))))

(fn ConstructionScript
  (|CallParentFunction))