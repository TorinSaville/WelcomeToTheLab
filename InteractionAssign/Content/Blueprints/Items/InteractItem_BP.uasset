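; Base-style interactable item Blueprint that bobs in the world and shows an interact prompt when the player character is near.
; Overlap with InteractionAssignCharacter sets its ItemIsNear flag and creates an InteractPrompt_BP widget, passed through SetItemNameForDisplay, which is an empty hook here.
; End overlap clears the flag and removes all top-level prompt widgets.
; Tick plays the Bob_UpDown timeline, whose output feeds a local location offset.
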(event Collision|EventActorBeginOverlap
  (params (OtherActor :type Actor%20Object%20Reference))
  (bind _asinteraction_assign_character (Utilities|Casting|CastToInteractionAssignCharacter OtherActor))
  (Variables|/Script/InteractionAssign.InteractionAssignCharacter|SetitemIsNear _asinteraction_assign_character true)
  (bind _returnvalue (UserInterface|CreateWidget "/Game/UI/Widgets/InteractPrompt_BP.InteractPrompt_BP_C"))
  (CallFunction|SetItemNameforDisplay _returnvalue)
  (UserInterface|Viewport|AddtoViewport _returnvalue 0))

(event EventTick
  (params (DeltaSeconds :type Float%20%28single-precision%29))
  (bind _updown (Timeline|Bob_UpDown Play)
    (:Update
      (Transformation|AddActorLocalOffset _updown false false))))

(event Collision|EventActorEndOverlap
  (params (OtherActor :type Actor%20Object%20Reference))
  (bind _asinteraction_assign_character (Utilities|Casting|CastToInteractionAssignCharacter OtherActor))
  (Variables|/Script/InteractionAssign.InteractionAssignCharacter|SetitemIsNear _asinteraction_assign_character false)
  (bind _foundwidgets (Widget|GetAllWidgetsOfClass "/Game/UI/Widgets/InteractPrompt_BP.InteractPrompt_BP_C" true))
  (for _array_element _foundwidgets
    (Widget|RemovefromParent _array_element)))

(fn ConstructionScript)

(fn SetItemNameforDisplay
  (params (Widget%20Ref :type Interact%20Prompt%20BP%20Object%20Reference)))