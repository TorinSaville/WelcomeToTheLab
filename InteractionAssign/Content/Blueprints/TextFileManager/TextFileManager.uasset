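; Session logger that records one play session's stats to a timestamped CSV file in the project's CVSFiles folder.
; BeginPlay starts a comma-separated string with date and time, and caches the player character.
; EndPlay appends game time, end time, pickup counts, damage and healing, and exit reason (quit, loss or win), then saves via SaveArrayText.
; The stat variables are only read here, never updated.
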(event EventEndPlay
  (params (EndPlayReason :type EEndPlayReason%20Enum :default "Destroyed"))
  (CallFunction|GameTime)
  (CallFunction|EndPoint)
  (CallFunction|PickUps)
  (CallFunction|Health)
  (CallFunction|Exit)
  (CallFunction|SaveFile))

(event EventBeginPlay
  (CallFunction|StartPoint)
  (bind _asbp_third_person_character (Utilities|Casting|CastToBP_ThirdPersonCharacter (Game|GetPlayerCharacter 0)))
  (Variables|Default|SetPlayerRef _asbp_third_person_character))

(fn ConstructionScript)

(fn StartPoint
  (Variables|File|SetDataElement (Utilities|String|Append (Utilities|GetDate) (Utilities|GetTime))))

(fn SaveFile
  (bind _filetext (Variables|File|GetFileText))
  (Utilities|Array|Add _filetext (Variables|File|GetDataElement))
  (Class|TextFileManager|SaveArrayText (Utilities|GetTextFileDir) (Utilities|CreateFileName) _filetext false))

(fn EndPoint
  (Variables|File|SetDataElement (Utilities|String|Append (Variables|File|GetDataElement) (Utilities|GetTime) ",")))

(fn PickUps
  (bind _damagepu (Variables|PickUps|GetDamagePU))
  (bind _healthpu (Variables|PickUps|GetHealthPU))
  (bind _staminapu (Variables|PickUps|GetStaminaPU))
  (Variables|File|SetDataElement (Utilities|String|Append (Variables|File|GetDataElement) (Utilities|GetPickUps _damagepu) (Utilities|GetPickUps _healthpu) (Utilities|GetPickUps _staminapu) (Utilities|GetTotalPickUps _damagepu _healthpu _staminapu) ",")))

(fn GameTime
  (Variables|File|SetDataElement (Utilities|String|Append (Variables|File|GetDataElement) (Utilities|String|ToString(Text) (Utilities|Text|FormatText "{Min}:{Sec}," (Variables|GameTime|GetGameMinutes) (Variables|GameTime|GetGameSeconds))))))

(fn Health
  (Variables|File|SetDataElement (Utilities|String|Append (Variables|File|GetDataElement) (Utilities|GetHealth (Variables|Health|GetDamageTaken)) (Utilities|GetHealth (Variables|Health|GetHealthHealed)) ",")))

(fn ExitSetting
  (if (== (Variables|Exit|GetExitCondition) 0)
    (Variables|Exit|SetExitReason "PlayerQuit")
    (elif (== (Variables|Exit|GetExitCondition) 1)
      (Variables|Exit|SetExitReason "PlayerLoss")
      (else
        (Variables|Exit|SetExitReason "PlayerWin")))))

(fn Exit
  (CallFunction|ExitSetting)
  (Variables|File|SetDataElement (Utilities|String|Append (Variables|File|GetDataElement) (Utilities|String|ToString(Text) (Utilities|Text|FormatText "{0}," (Variables|Exit|GetExitReason))))))